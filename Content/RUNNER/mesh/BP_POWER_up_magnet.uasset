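; Magnet power-up pickup for the runner game that, on overlap with BP_runner, plays a sound, destroys and hides itself, and switches on the runner's magnet flag.
; If the magnet was inactive, it sets the game mode's MagnetTIMER and decrements it in a zero-delay loop.
; A separate fixed Delay is meant to clear the flag, although DestroyActor has already run by then.
; Overlapping a BP_wall also destroys the pickup.
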(event `self.ReceiveActorBeginOverlap`
  (params (OtherActor :type "Actor Object Reference"))
  (`|ExecutionSequence`
    (:`then_0`
      (bind _asbp_runner (cast `/Game/RUNNER/BLUEPRINT/BP_runner` OtherActor))
      (bind _asbp_runner_gm (cast `/Game/RUNNER/BLUEPRINT/BP_RUNNER_GM` (`GameplayStatics.GetGameMode`)))
      (`GameplayStatics.PlaySound2D` "/Game/RUNNER/mesh/350874__cabled_mess__coin_c_08.350874__cabled_mess__coin_c_08" 1.0 1.0 0.0 null null)
      (`self.K2_DestroyActor`)
      (`self.SetActorHiddenInGame` true)
      (if (not (`/Game/RUNNER/BLUEPRINT/BP_runner.IS MAGNET  active?` _asbp_runner))
        (set `/Game/RUNNER/BLUEPRINT/BP_runner.IS MAGNET  active?` true _asbp_runner)
        (set `/Game/RUNNER/BLUEPRINT/BP_RUNNER_GM.magnet_TIMER` 6.0 _asbp_runner_gm)
        (`KismetSystemLibrary.PrintString` "MAGNET IS ACTIVE" true false)
        (`|ExecutionSequence`
          (:`then_0`
            (`/Game/RUNNER/INPUT/loop_DELAY.LOOP_WITH_DELAY` 0 5
              (:`loop body`
                (bind _result (`/Engine/EditorBlueprintResources/StandardMacros.DecrementFloat` (`/Game/RUNNER/BLUEPRINT/BP_RUNNER_GM.magnet_TIMER` _asbp_runner_gm))
                  (:`  `
                    (bind _output_get (set `/Game/RUNNER/BLUEPRINT/BP_RUNNER_GM.magnet_TIMER` (`KismetMathLibrary.FMax` _result) _asbp_runner_gm))
                    (`KismetSystemLibrary.PrintString` (`KismetStringLibrary.Conv_DoubleToString` _output_get) true false (struct :`R` 1.0 :`A` 1.0)))))))
          (:`then_1`
            (`KismetSystemLibrary.Delay` 5.2)
            (`KismetSystemLibrary.PrintString` "Hello")
            (bind _asbp_runner_2 (cast `/Game/RUNNER/BLUEPRINT/BP_runner` (`GameplayStatics.GetPlayerCharacter` 0)))
            (set `/Game/RUNNER/BLUEPRINT/BP_runner.IS MAGNET  active?` false _asbp_runner_2)
            (`KismetSystemLibrary.PrintString` "MAGNET IN ACTIVE" true false)
            (`self.K2_DestroyActor`)))))
    (:`then_1`
      (cast `/Game/RUNNER/obstecales/BP_wall` OtherActor)
      (`self.K2_DestroyActor`))))

(fn `UserConstructionScript`)