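; Floor tile for an endless runner that populates itself with randomly placed obstacles, coins and periodic power-ups.
; The construction script builds spawn points across the lanes from arrow components, then attaches child actors at shuffled points.
; Power-ups appear once the game mode's floor count passes a threshold, which then resets.
; Box overlap asks the game mode to extend the floor, slightly raises the runner's clamped speed and adds multiplier-based score.
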(event `self.Box.OnComponentBeginOverlap`
  (params (OverlappedComponent :type "PrimitiveComponent Object Reference") (OtherActor :type "Actor Object Reference") (OtherComp :type "PrimitiveComponent Object Reference") (OtherBodyIndex :type Integer) (bFromSweep :type Boolean) (SweepResult :type "HitResult Structure (by ref)"))
  ;[1 1 1] floor
  (bind _asbp_runner_gm (cast `/Game/RUNNER/BLUEPRINT/BP_RUNNER_GM` (`GameplayStatics.GetGameMode`)))
  (`/Game/RUNNER/BLUEPRINT/BP_RUNNER_GM.extent floor` _asbp_runner_gm)
  (bind _asbp_runner (cast `/Game/RUNNER/BLUEPRINT/BP_runner` (`GameplayStatics.GetPlayerCharacter` 0)))
  (bind _charactermovement (`Character.CharacterMovement` _asbp_runner))
  (set `CharacterMovementComponent.MaxWalkSpeed` (`KismetMathLibrary.FClamp` (* (`CharacterMovementComponent.MaxWalkSpeed` _charactermovement) 1.001) 700.0 2000.0) _charactermovement)
  ;[1 1 1] current score
  (bind _asbp_runner_gm_2 (cast `/Game/RUNNER/BLUEPRINT/BP_RUNNER_GM` (`GameplayStatics.GetGameMode`)))
  (set `/Game/RUNNER/BLUEPRINT/BP_RUNNER_GM.CURRENT POINTS` (+ (* (`/Game/RUNNER/BLUEPRINT/BP_RUNNER_GM. points multi` _asbp_runner_gm_2) 1) (`/Game/RUNNER/BLUEPRINT/BP_RUNNER_GM.CURRENT POINTS` _asbp_runner_gm_2)) _asbp_runner_gm_2))

(fn `coin spawn points`
  (for _array_element (`self.lane position`)
    (for _index (range 10)
      (bind _returnvalue (`AddComponent|NODE_AddArrowComponent-1` :`RelativeTransform` (`KismetMathLibrary.MakeTransform` (`KismetMathLibrary.MakeVector` (* _index 75.0) _array_element))))
      (`ArrowComponent.SetArrowColor` _returnvalue (struct :`R` 0.095265 :`G` 1.0 :`B` 0.012008 :`A` 1.0))
      (`KismetArrayLibrary.Array_Add` (`self.CS spawn point`) (`SceneComponent.K2_GetComponentToWorld` _returnvalue)))))

(fn `get attach point`
  (returns (ReturnValue :type "Transform Structure"))
  (return (`SceneComponent.K2_GetComponentToWorld` (`self.Arrow`))))

(fn `PMAGNET_SPAWN`
  (for _array_element (`self.lane position`)
    (for _index (range 1 3)
      (bind _returnvalue (`AddComponent|NODE_AddArrowComponent-2` :`RelativeTransform` (`KismetMathLibrary.MakeTransform` (`KismetMathLibrary.MakeVector` (* _index 250.0) _array_element))))
      (`ArrowComponent.SetArrowColor` _returnvalue (struct :`R` 1.0 :`G` 0.755585 :`A` 1.0))
      (`KismetArrayLibrary.Array_Add` (`self.PSPAWN_POINT`) (`SceneComponent.K2_GetComponentToWorld` _returnvalue)))))

(fn `setup spawn point`
  (for _array_element (`self.lane position`)
    (for _index (range 1)
      (bind _returnvalue (`AddComponent|NODE_AddArrowComponent-0` :`RelativeTransform` (`KismetMathLibrary.MakeTransform` (`KismetMathLibrary.MakeVector` (* _index 650.0) _array_element))))
      (`KismetArrayLibrary.Array_Add` (`self.spwan points`) (`SceneComponent.K2_GetComponentToWorld` _returnvalue)))))

(fn `spawn coin`
  (bind _output_get (set `self.Random spawn points` (`self.CS spawn point`)))
  (`KismetArrayLibrary.Array_Shuffle` _output_get)
  (for _index (range (+ (`KismetMathLibrary.RandomIntegerInRange` 5 8) 1))
    (switch `int` 0
      (:`0`
        (`AddComponent|NODE_AddChildActorComponent-4` :`RelativeTransform` (`KismetMathLibrary.MakeRelativeTransform` (`|GetArrayItem` (`self.Random spawn points`) _index) (`self.GetTransform`)))))))

(fn `spawn obstacles`
  (bind _output_get (set `self.Random spawn points` (`self.spwan points`)))
  (`KismetArrayLibrary.Array_Shuffle` _output_get)
  (for _index (range (+ (`KismetMathLibrary.RandomIntegerInRange` 0 1) 1))
    (switch `int` (`KismetMathLibrary.RandomIntegerInRange` 0 1)
      (:`0`
        (bind _returnvalue (`KismetMathLibrary.MakeRelativeTransform` (`|GetArrayItem` (`self.Random spawn points`) _index) (`self.GetTransform`)))
        (`AddComponent|NODE_AddChildActorComponent-0` :`RelativeTransform` _returnvalue))
      (:`1`
        (`AddComponent|NODE_AddChildActorComponent-1` :`RelativeTransform` _returnvalue)))))

(fn `SPAWN_POWER_up`
  (bind _asbp_runner_gm (cast `/Game/RUNNER/BLUEPRINT/BP_RUNNER_GM` (`GameplayStatics.GetGameMode`)))
  (if (> (`/Game/RUNNER/BLUEPRINT/BP_RUNNER_GM.FLOOR_COUNT` _asbp_runner_gm) 5)
    (bind _output_get (set `self.Random spawn points` (`self.PSPAWN_POINT`)))
    (`KismetArrayLibrary.Array_Shuffle` _output_get)
    (switch `int` 0
      (:`0`
        (`AddComponent|NODE_AddChildActorComponent-5` :`RelativeTransform` (`KismetMathLibrary.MakeRelativeTransform` (`|GetArrayItem` (`self.Random spawn points`)) (`self.GetTransform`)))
        (set `/Game/RUNNER/BLUEPRINT/BP_RUNNER_GM.FLOOR_COUNT` 0 _asbp_runner_gm)))))

(fn `UserConstructionScript`
  (`self.setup spawn point`)
  (`self.spawn obstacles`)
  (`self.coin spawn points`)
  (`self.spawn coin`)
  (`self.PMAGNET_SPAWN`)
  (`self.SPAWN_POWER_up`))