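; BP_RUNNER_GM is the endless runner's manager Blueprint, which builds the floor track and restores the saved coin count.
; BeginPlay spawns the initial tiles, reloading COIN from the SAVE_COIN slot on every loop pass.
; AddFloor chains each ENDLESS_FLOOR to the previous tile's attach point, tracking it in FloorTiles and FLOORCOUNT.
; ExtentFloor appends a tile and destroys the oldest once the array exceeds the starting count plus a buffer.
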(event `self.ReceiveBeginPlay`
  ;[1 1 1] floor spawning
  (for _ (range (`self.NO of tiles`))
    (`self.add floor`)
    (bind _returnvalue (`GameplayStatics.LoadGameFromSlot` "SAVE_COIN"))
    (bind _asbp_save_score (cast `/Game/RUNNER/BLUEPRINT/BP_SAVE_SCORE` _returnvalue))
    (set `self.COIN` (`/Game/RUNNER/BLUEPRINT/BP_SAVE_SCORE.SAVE_COIN` _asbp_save_score))))

(fn `add floor`
  (bind _returnvalue (`|SpawnActorFromClass` "/Game/RUNNER/BLUEPRINT/ENDLESS_FLOOR.ENDLESS_FLOOR_C" (`self.floor attach point`) "Undefined" "MultiplyWithRoot" null null))
  (bind _returnvalue_2 (`/Game/RUNNER/BLUEPRINT/ENDLESS_FLOOR.get attach point` _returnvalue))
  (set `self.floor attach point` _returnvalue_2)
  (`KismetArrayLibrary.Array_Add` (`self.floor tiles`) _returnvalue)
  (bind _result (`/Engine/EditorBlueprintResources/StandardMacros.IncrementInt` (`self.FLOOR_COUNT`))
    (:`  `
      (set `self.FLOOR_COUNT` _result))))

(fn `extent floor`
  (bind _floor_tiles (`self.floor tiles`))
  (bind _output (`|GetArrayItem` _floor_tiles))
  ;[1 1 1] floor extent
  (`self.add floor`)
  (if (> (`KismetArrayLibrary.Array_Length` (`self.floor tiles`)) (+ (`self.NO of tiles`) 10))
    (`self.K2_DestroyActor` _output)
    (`KismetArrayLibrary.Array_RemoveItem` _floor_tiles _output)))

(fn `UserConstructionScript`)