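; BP_wall is an obstacle for the runner game that the player character must slide through to survive.
; When its Box component is overlapped by BP_runner, it checks the runner's IsSLIDING flag.
; If the runner is not sliding, it calls DEATH on the runner, waits briefly, then pauses the game.
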(event `self.Box.OnComponentBeginOverlap`
  (params (OverlappedComponent :type "PrimitiveComponent Object Reference") (OtherActor :type "Actor Object Reference") (OtherComp :type "PrimitiveComponent Object Reference") (OtherBodyIndex :type Integer) (bFromSweep :type Boolean) (SweepResult :type "HitResult Structure (by ref)"))
  (bind _asbp_runner (cast `/Game/RUNNER/BLUEPRINT/BP_runner` OtherActor))
  (if (not (`/Game/RUNNER/BLUEPRINT/BP_runner.isSLIDING` _asbp_runner))
    (`/Game/RUNNER/BLUEPRINT/BP_runner.DEATH` _asbp_runner)
    (`KismetSystemLibrary.Delay` 1.0)
    (`GameplayStatics.SetGamePaused` true)))

(fn `UserConstructionScript`
  (`parent.UserConstructionScript`))